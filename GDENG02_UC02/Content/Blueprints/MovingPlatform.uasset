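; Moving platform actor that slides its Cube component back and forth between a start and an end location.
; BeginPlay stores the Cube's relative location and derives the end by adding Distance on Y, which also doubles the start's X and Z.
; Each Tick steps a clamped lerp alpha by AlphaMultiplier times delta time, with HasReachedEnd flipping direction at either limit.
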(event `self.ReceiveBeginPlay`
  (set `self.StartLocation` (`SceneComponent.RelativeLocation` (`self.Cube`)))
  (`self.GetEndLocation`))

(event `self.ReceiveTick`
  (params (DeltaSeconds :type "Float (single-precision)"))
  (`self.MovePlatform` DeltaSeconds))

(fn `GetEndLocation`
  (set `self.EndLocation` (+ (`self.StartLocation`) (`KismetMathLibrary.MakeVector` (.x (`self.StartLocation`)) (`self.Distance`) (.z (`self.StartLocation`))))))

(fn `MovePlatform`
  (params (deltaSeconds :type "Float (double-precision)"))
  (if (`self.hasReachedEnd`)
    (`self.MoveToStart` deltaSeconds)
    (else
      (`self.MoveToEnd` deltaSeconds))))

(fn `MoveToEnd`
  (params (deltaSeconds :type "Float (double-precision)"))
  (set `self.AlphaLerp` (`KismetMathLibrary.FClamp` (+ (* (`self.AlphaMultiplier`) deltaSeconds) (`self.AlphaLerp`))))
  (`SceneComponent.K2_SetRelativeLocation` (`self.Cube`) (`KismetMathLibrary.VLerp` (`self.StartLocation`) (`self.EndLocation`) (`self.AlphaLerp`)) false false)
  (if (== (`self.AlphaLerp`) 1.0)
    (set `self.hasReachedEnd` true)))

(fn `MoveToStart`
  (params (deltaSeconds :type "Float (double-precision)"))
  (set `self.AlphaLerp` (`KismetMathLibrary.FClamp` (- (`self.AlphaLerp`) (* (`self.AlphaMultiplier`) deltaSeconds))))
  (`SceneComponent.K2_SetRelativeLocation` (`self.Cube`) (`KismetMathLibrary.VLerp` (`self.StartLocation`) (`self.EndLocation`) (`self.AlphaLerp`)) false false)
  (if (== (`self.AlphaLerp`) 0.0)
    (set `self.hasReachedEnd` false)))

(fn `UserConstructionScript`)