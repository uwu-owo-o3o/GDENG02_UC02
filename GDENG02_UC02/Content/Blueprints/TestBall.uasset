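; TestBall is a player ball that rolls, jumps and collects Ring actors up to a maximum count.
; MoveX and MoveY nudge the sphere's relative rotation and location in fixed steps without sweep, BallJump applies an upward force, and StopMovement toggles physics off and on.
; Each tick, it finds overlapping WorldStatic actors named "Ring", recolors and counts uncollected ones, and snaps the camera to a fixed offset from the sphere.
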(event `self.ReceiveBeginPlay`)

(event `self.ReceiveTick`
  (params (DeltaSeconds :type "Float (single-precision)"))
  (`self.CollectRing`)
  (`self.CameraFollow`))

(fn `AddRing`
  (params (otherActor :type "Actor Object Reference"))
  (bind _asring (cast `/Game/Blueprints/Ring` otherActor))
  (if (not (`/Game/Blueprints/Ring.IsCollected` _asring))
    (`/Game/Blueprints/Ring.ChangeColor` _asring)
    (if (< (`self.NumCollectedRings`) (`self.MaxRingsToCollect`))
      (set `self.NumCollectedRings` (+ (`self.NumCollectedRings`) 1))
      (set `/Game/Blueprints/Ring.IsCollected` true _asring))))

(fn `BallJump`
  (params (bool :type Boolean))
  (`KismetSystemLibrary.PrintText` "JUMP!")
  (`PrimitiveComponent.AddForce` (`self.Sphere`) (0.0 0.0 4000000.0) "None" false))

(fn `CameraFollow`
  (`SceneComponent.K2_SetRelativeLocation` (`self.Camera`) (+ (`SceneComponent.RelativeLocation` (`self.Sphere`)) (-850.0 0.0 250.0)) false false))

(fn `CollectRing`
  (bind _sphere (`self.Sphere`))
  (bind (_outactors _returnvalue) (`KismetSystemLibrary.ComponentOverlapActors` _sphere (`SceneComponent.GetRelativeTransform` _sphere) (`|MakeArray` "ObjectTypeQuery1" :!type "EObjectTypeQuery Enum")))
  (if _returnvalue
    (for _array_element _outactors
      (if (`KismetStringLibrary.Contains` (`KismetSystemLibrary.GetDisplayName` _array_element) "Ring")
        (`self.AddRing` _array_element)))))

(fn `Move Y`
  (params (offset :type "Float (double-precision)"))
  (bind _sphere (`self.Sphere`))
  (bind _sphere_2 (`self.Sphere`))
  (bind _sphere_3 (`self.Sphere`))
  (bind _sphere_4 (`self.Sphere`))
  (if (== offset 1.0)
    ;[1 1 1] North Movement
    (`SceneComponent.K2_SetRelativeRotation` _sphere_2 (`KismetMathLibrary.MakeRotator` (.roll (`SceneComponent.RelativeRotation` _sphere_2)) (+ (.pitch (`SceneComponent.RelativeRotation` _sphere_2)) 5.0) (.yaw (`SceneComponent.RelativeRotation` _sphere_2))) false false)
    (`SceneComponent.K2_SetRelativeLocation` _sphere_3 (`KismetMathLibrary.MakeVector` (+ (.x (`SceneComponent.RelativeLocation` _sphere_3)) 5.0) (.y (`SceneComponent.RelativeLocation` _sphere_3)) (.z (`SceneComponent.RelativeLocation` _sphere_3))) false false)
    (else
      ;[1 1 1] North Movement
      (`SceneComponent.K2_SetRelativeRotation` _sphere (`KismetMathLibrary.MakeRotator` (.roll (`SceneComponent.RelativeRotation` _sphere)) (+ (.pitch (`SceneComponent.RelativeRotation` _sphere)) -5.0) (.yaw (`SceneComponent.RelativeRotation` _sphere))) false false)
      (`SceneComponent.K2_SetRelativeLocation` _sphere_4 (`KismetMathLibrary.MakeVector` (+ (.x (`SceneComponent.RelativeLocation` _sphere_4)) -5.0) (.y (`SceneComponent.RelativeLocation` _sphere_4)) (.z (`SceneComponent.RelativeLocation` _sphere_4))) false false))))

(fn `MoveX`
  (params (offset :type "Float (double-precision)"))
  (bind _sphere (`self.Sphere`))
  (bind _sphere_2 (`self.Sphere`))
  (bind _sphere_3 (`self.Sphere`))
  (bind _sphere_4 (`self.Sphere`))
  (if (== offset 1.0)
    ;[1 1 1] Right Movement
    (`SceneComponent.K2_SetRelativeRotation` _sphere_4 (`KismetMathLibrary.MakeRotator` (+ (.roll (`SceneComponent.RelativeRotation` _sphere_4)) 5.0) (.pitch (`SceneComponent.RelativeRotation` _sphere_4)) (.yaw (`SceneComponent.RelativeRotation` _sphere_4))) false false)
    (`SceneComponent.K2_SetRelativeLocation` _sphere_2 (`KismetMathLibrary.MakeVector` (.x (`SceneComponent.RelativeLocation` _sphere_2)) (+ (.y (`SceneComponent.RelativeLocation` _sphere_2)) 5.0) (.z (`SceneComponent.RelativeLocation` _sphere_2))) false false)
    (else
      ;[1 1 1] Left Movement
      (`SceneComponent.K2_SetRelativeRotation` _sphere (`KismetMathLibrary.MakeRotator` (+ (.roll (`SceneComponent.RelativeRotation` _sphere)) -5.0) (.pitch (`SceneComponent.RelativeRotation` _sphere)) (.yaw (`SceneComponent.RelativeRotation` _sphere))) false false)
      (`SceneComponent.K2_SetRelativeLocation` _sphere_3 (`KismetMathLibrary.MakeVector` (.x (`SceneComponent.RelativeLocation` _sphere_3)) (+ (.y (`SceneComponent.RelativeLocation` _sphere_3)) -5.0) (.z (`SceneComponent.RelativeLocation` _sphere_3))) false false))))

(fn `StopMovement`
  (bind _sphere (`self.Sphere`))
  (`PrimitiveComponent.SetSimulatePhysics` _sphere false)
  (`PrimitiveComponent.SetSimulatePhysics` _sphere true))

(fn `UserConstructionScript`)