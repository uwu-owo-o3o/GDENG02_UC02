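; WinFlag is a goal actor that lets the player ball win once it has collected all of its rings.
; Every tick it reads the player TestBall's ring count and switches its Cylinder to a green material when that count equals the maximum.
; On overlap, it filters for display names containing "Ball", casts to TestBall, and prints either a win or a not-enough-rings message.
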(event `self.ReceiveActorBeginOverlap`
  (params (OtherActor :type "Actor Object Reference"))
  (`self.CheckWinCondition` OtherActor))

(event `self.ReceiveTick`
  (params (DeltaSeconds :type "Float (single-precision)"))
  (`self.ChangeColor`))

(fn `ChangeColor`
  (bind _astest_ball (cast `/Game/Blueprints/TestBall` (`GameplayStatics.GetPlayerPawn` 0)))
  (if (== (`/Game/Blueprints/TestBall.NumCollectedRings` _astest_ball) (`/Game/Blueprints/TestBall.MaxRingsToCollect` _astest_ball))
    (`PrimitiveComponent.SetMaterial` (`self.Cylinder`) 0 "/Game/Material/GreenMaterial.GreenMaterial")))

(fn `CheckWinCondition`
  (params (otherActor :type "Object Object Reference"))
  (if (`KismetStringLibrary.Contains` (`KismetSystemLibrary.GetDisplayName` otherActor) "Ball")
    (bind _astest_ball (cast `/Game/Blueprints/TestBall` otherActor))
    (if (== (`/Game/Blueprints/TestBall.NumCollectedRings` _astest_ball) (`/Game/Blueprints/TestBall.MaxRingsToCollect` _astest_ball))
      (`KismetSystemLibrary.PrintText` "YOU WIN!")
      (else
        (`KismetSystemLibrary.PrintText` "NOT ENOUGH RINGS!")))))

(fn `UserConstructionScript`)